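; BP_BaseButton is a base button Blueprint that asks a spawner to spawn a given class when interacted with.
; On BeginPlay it casts its Widget component's user widget to WBP_TextButton and sets the label text from NumbButton.
; InfoSpawn stores the spawner reference and the class, and Interact passes that class to the spawner's Spawn call.
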(event `self.ReceiveBeginPlay`
  (bind _aswbp_text_button (cast `/Game/Prodject/UI/WBP_TextButton` (`WidgetComponent.GetUserWidgetObject` (`self.Widget`))))
  (`TextBlock.SetText` (`/Game/Prodject/UI/WBP_TextButton.TextBlock_25` _aswbp_text_button) (`self.NumbButton`)))

(event `InfoSpawn`
  (params (Spawn :type "/Game/Prodject/Blueprints/Button/BP_Spawn Object Reference") (Class :type "Actor Class Reference"))
  (set `self.Spawn` Spawn)
  (set `self.Class` Class))

(event `/Game/Prodject/Blueprints/Button/BP_Communication.Interact`
  (`/Game/Prodject/Blueprints/Button/BP_Spawn.Spawn` (`self.Spawn`) (`self.Class`)))

(fn `UserConstructionScript`)