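; Base animal character Blueprint that drives AI movement toward a target actor and back toward a spawn actor.
; After a short BeginPlay delay, MoveEvent issues AI MoveTo, then sets timers depending on stop and back-move conditions.
; StopMove halts character movement and BackMove heads for the spawn actor, each scheduling a follow-up timer.
; EndMove sets a flag that blocks further move orders and stops movement.
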(event `self.ReceiveBeginPlay`
  (`KismetSystemLibrary.Delay` 0.2)
  (`self.MoveEvent`))

(event `MoveEvent`
  (if (not (`self.End Move`))
    (`|AIMoveTo` self (0.0 0.0 0.0) (`self.Target Actor`)
      (:`then`
        (if (`self.Stop Move`)
          (`KismetSystemLibrary.K2_SetTimerDelegate` (`|CreateDelegate` :!event `StopMove`) 1.0))
        (if (`self.Back Move`)
          (`KismetSystemLibrary.K2_SetTimerDelegate` (`|CreateDelegate` :!event `BackMove`) 1.0))))))

(event `StopMove`
  (`NavMovementComponent.StopActiveMovement` (`self.CharacterMovement`))
  (`KismetSystemLibrary.K2_SetTimerDelegate` (`|CreateDelegate` :!event `MoveEvent`) 0.5))

(event `BackMove`
  (if (not (`self.End Move`))
    (`|AIMoveTo` self (0.0 0.0 0.0) (`self.Spawn Actor`)
      (:`then`
        (`KismetSystemLibrary.K2_SetTimerDelegate` (`|CreateDelegate` :!event `MoveEvent`) 0.5)))))

(event `EndMove`
  (set `self.End Move` true)
  (`NavMovementComponent.StopActiveMovement` (`self.CharacterMovement`)))

(fn `UserConstructionScript`
  (`parent.UserConstructionScript`))